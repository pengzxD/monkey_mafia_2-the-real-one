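; Director Blueprint that tracks the zombie population (Bp_mexican) and fulfils spawn requests from horde spawners (Bp_horedSpawner).
; On BeginPlay it registers all existing zombies and spawners, binding to their killed and spawn-request events.
; Killed zombies leave the tracked array, whose size limits each request against MaxMexican.
; New zombies spawn at random reachable points near the requested location and are registered the same way.
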(event `self.ReceiveBeginPlay`
  (`|ExecutionSequence`
    (:`then_0`
      (bind _outactors (`GameplayStatics.GetAllActorsOfClass` "/Game/Game/MexicanAI/bp_mexican.bp_mexican_C"))
      (for _array_element _outactors
        (`self.OnZombieSpawn` _array_element)))
    (:`then_1`
      (bind _outactors_2 (`GameplayStatics.GetAllActorsOfClass` "/Game/Game/Director/bp_horedSpawner.bp_horedSpawner_C"))
      (for _array_element_2 _outactors_2
        (`self.OnHoredSpawnerSpawn` _array_element_2)))))

(fn `On Zombie Killed`
  (params (Mexican :type "/Game/Game/MexicanAI/bp_mexican Object Reference"))
  (`KismetArrayLibrary.Array_RemoveItem` (`self.Mexican`) Mexican))

(fn `OnHoredSpawnerSpawn`
  (params (HoredSpawner :type "/Game/Game/Director/bp_horedSpawner Object Reference"))
  (`KismetArrayLibrary.Array_Add` (`self.Hored Spawner`) HoredSpawner)
  (add `/Game/Game/Director/bp_horedSpawner.RequestSpawn` HoredSpawner (`|CreateDelegate` :!event `OnZombieSpawnRequested`)))

(fn `OnZombieSpawn`
  (params (Mexican :type "/Game/Game/MexicanAI/bp_mexican Object Reference"))
  (`KismetArrayLibrary.Array_Add` (`self.Mexican`) Mexican)
  (add `/Game/Game/MexicanAI/bp_mexican.OnKilled` Mexican (`|CreateDelegate` :!event `On Zombie Killed`)))

(fn `OnZombieSpawnRequested`
  (params (count :type Integer) (location :type "Vector Structure"))
  (for _ (range 1 (+ (`KismetMathLibrary.Min` count (- (`self.maxMexican`) (`KismetArrayLibrary.Array_Length` (`self.Mexican`)))) 1))
    (bind _returnvalue (`|SpawnActorFromClass` "/Game/Game/MexicanAI/bp_mexican.bp_mexican_C" (`KismetMathLibrary.MakeTransform` (+ (`NavigationSystemV1.K2_GetRandomReachablePointInRadius` (`local.location`) 200.0 null null) (0.0 0.0 88.0))) "Undefined" "OverrideRootScale" null null))
    (`self.OnZombieSpawn` _returnvalue)))

(fn `UserConstructionScript`)