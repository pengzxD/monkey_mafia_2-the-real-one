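; Character Blueprint for a Mexican AI character that adds random variety at spawn and ragdolls when killed.
; BeginPlay randomizes mesh scale per axis, facing yaw and max walk speed.
; The kill event stops the AI brain logic, switches the mesh to physics ragdoll and changes the capsule's collision profile.
; After a short delay it fires the OnKilled dispatcher and destroys the actor.
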(event `self.ReceiveBeginPlay`
  (bind _returnvalue (`KismetMathLibrary.RandomFloatInRange` 0.9 1.1))
  (`SceneComponent.SetWorldScale3D` (`self.Mesh`) (`KismetMathLibrary.MakeVector` _returnvalue _returnvalue _returnvalue))
  (`self.K2_SetActorRotation` (`KismetMathLibrary.MakeRotator` 0.0 0.0 (`KismetMathLibrary.RandomFloatInRange` 0.0 360.0)))
  (set `CharacterMovementComponent.MaxWalkSpeed` (`KismetMathLibrary.RandomFloatInRange` 450.0 650.0) (`self.CharacterMovement`)))

(event `kill`
  (bind _mesh (`self.Mesh`))
  (`BrainComponent.StopLogic` (`AIController.BrainComponent` (`AIBlueprintHelperLibrary.GetAIController` self)) "")
  (`PrimitiveComponent.SetCollisionProfileName` _mesh "ragdoll" true)
  (`PrimitiveComponent.SetSimulatePhysics` _mesh true)
  (`PrimitiveComponent.SetCollisionProfileName` (`self.CapsuleComponent`) "NoCollsion" true)
  (`KismetSystemLibrary.Delay` 3.0)
  (`self.OnKilled` self)
  (`self.K2_DestroyActor`))

(fn `UserConstructionScript`)