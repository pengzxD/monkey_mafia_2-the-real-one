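; Horde spawner trigger actor that requests a randomly sized spawn when a FirstPersonCharacter enters its box.
; The overlap calls RequestSpawn with a count between the min and max horde size and the SpawnLocation component's world position, leaving the spawning itself outside this Blueprint.
; A short timer re-enables the box's collision, which is switched off on each trigger as a brief cooldown, so the spawner is reusable.
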(event `self.triggerBox.OnComponentBeginOverlap`
  (params (OverlappedComponent :type "PrimitiveComponent Object Reference") (OtherActor :type "Actor Object Reference") (OtherComp :type "PrimitiveComponent Object Reference") (OtherBodyIndex :type Integer) (bFromSweep :type Boolean) (SweepResult :type "HitResult Structure (by ref)"))
  (cast `/Game/Player/FirstPersonCharacter` OtherActor)
  (`PrimitiveComponent.SetCollisionProfileName` (`self.triggerBox`) "NoCollision" true)
  (`KismetSystemLibrary.K2_SetTimerDelegate` (delegate `enable trigger`) 1.0)
  (`self.RequestSpawn` (`KismetMathLibrary.RandomIntegerInRange` (`self.hored size min`) (`self.hored size max`)) (`SceneComponent.K2_GetComponentLocation` (`self.spawn_location`))))

(event `enable trigger`
  (`PrimitiveComponent.SetCollisionProfileName` (`self.triggerBox`) "trigger" true))

(fn `UserConstructionScript`)