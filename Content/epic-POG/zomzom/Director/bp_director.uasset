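; Director Blueprint that keeps a list of living Bp_mexican zombie actors.
; OnZombieSpawn adds a zombie to the list and binds an event to its OnKilled dispatcher, while OnZombieKilled removes a zombie from the list.
; BeginPlay gathers all existing Bp_mexican actors, but the loop that would register them through OnZombieSpawn is disconnected and never runs.
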(event `self.ReceiveBeginPlay`
  (bind _outactors (`GameplayStatics.GetAllActorsOfClass` "/Game/epic-POG/zomzom/ai_for_mexican/bp_mexican.bp_mexican_C")))

(fn `On Zombie Killed`
  (params (Mexican :type "/Game/epic-POG/zomzom/ai_for_mexican/bp_mexican Object Reference"))
  (`KismetArrayLibrary.Array_RemoveItem` (`self.Mexican`) Mexican))

(fn `OnZombieSpawn`
  (params (Mexican :type "/Game/epic-POG/zomzom/ai_for_mexican/bp_mexican Object Reference"))
  (`KismetArrayLibrary.Array_Add` (`self.Mexican`) Mexican)
  (add `/Game/epic-POG/zomzom/ai_for_mexican/bp_mexican.OnKilled` Mexican (`|CreateDelegate` :!event `On Zombie Killed`)))

(fn `UserConstructionScript`)